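; GM_Main is the main game mode, managing a red and a blue character that the player switches between on a grid-based level.
; On BeginPlay it finds BP_Level, spawns both characters at its start cells, links them with a BP_Line and possesses the one chosen by RedStart.
; Helper functions flip the active character and report the active and other character's references and row/column positions.
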(event EventBeginPlay
  (bind _returnvalue (Actor|GetActorOfClass "/Game/Top/BP/BP_Level.BP_Level_C"))
  (Variables|关卡|SetBP_Level _returnvalue)
  (CallFunction|FUNSpawnPCH))

(fn ConstructionScript)

(fn FUNSpawnPCH
  (bind (_red _blue _redrow _redcolumn _bluerow _bluecolumn) (Default|FUNGetStart (Variables|关卡|GetBP_Level)))
  (bind _returnvalue (Game|SpawnActorfromClass "/Game/Top/GamePlay/PCH_Main_Red.PCH_Main_Red_C" (Math|Transform|MakeTransform _red "0, 0, 0" "1,1,1") "Undefined" 0 _redrow _redcolumn 0))
  (bind _returnvalue_2 (Game|SpawnActorfromClass "/Game/Top/GamePlay/PCH_Main_Blue.PCH_Main_Blue_C" (Math|Transform|MakeTransform _blue "0, 0, 0" "1,1,1") "Undefined" 0 _bluerow _bluecolumn 0))
  (Variables|关卡|SetPCHRed _returnvalue)
  (Variables|关卡|SetPCHBlue _returnvalue_2)
  (Default|FUNPossess (select (Variables|Config|GetRedStart?) (Variables|关卡|GetPCHRed) (Variables|关卡|GetPCHBlue)) true)
  (Variables|关卡|SetNowPCHRed (Variables|Config|GetRedStart?))
  (Game|SpawnActorfromClass "/Game/Top/BP/BP_Line.BP_Line_C" (Math|Transform|MakeTransform "0, 0, 0" "0, 0, 0" "1,1,1") "Undefined" 0 (Variables|关卡|GetPCHBlue) (Variables|关卡|GetPCHRed) 0))

(fn FUNSwitchPCH
  (Variables|关卡|SetNowPCHRed (not (Variables|关卡|GetNowPCHRed)))
  (Default|FUNPossess (.PCH (CallFunction|FUNGetNowPCH)) true))

(fn FUNGetNowPCH
  (bind _pchred (Variables|关卡|GetPCHRed))
  (bind _pchblue (Variables|关卡|GetPCHBlue))
  (return (select (Variables|关卡|GetNowPCHRed) _pchred _pchblue) (select (Variables|关卡|GetNowPCHRed) _pchblue _pchred)))

(fn FUNGetNowPCHLocation
  (bind (_pch _other) (CallFunction|FUNGetNowPCH))
  (return (Variables|/Game/Top/GamePlay/PCH_Main.PCH_Main_C|GetNowRow _pch) (Variables|/Game/Top/GamePlay/PCH_Main.PCH_Main_C|GetNowColumn _pch) (Variables|/Game/Top/GamePlay/PCH_Main.PCH_Main_C|GetNowRow _other) (Variables|/Game/Top/GamePlay/PCH_Main.PCH_Main_C|GetNowColumn _other)))